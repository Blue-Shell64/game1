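; BP_Player is the player character, handling movement, look, health damage and respawning.
; On BeginPlay it adds the IMC_Player Enhanced Input mapping context and stores its starting transform, with move and look actions driving movement input and controller rotation.
; Capsule hits on components tagged "pain1" or "pain2" subtract health, heavier for pain1.
; When health runs out, the death event returns the player to the stored transform and restores health.
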(event `self.ReceiveBeginPlay`
  (`EnhancedInputSubsystemInterface.AddMappingContext` (pcsubsystem `EnhancedInputLocalPlayerSubsystem` (`GameplayStatics.GetPlayerController` 0)) "/Game/Blueprints/IMC_Player.IMC_Player" 0 (struct))
  (set `self.startPos` (`self.GetTransform`)))

(event `EnhancedInput|/Game/Blueprints/IA_Move`
  (params (ActionValue :type "Vector2D Structure") (ElapsedSeconds :type "Float (double-precision)") (TriggeredSeconds :type "Float (double-precision)") (InputAction :type "InputAction Object Reference" :default "/Game/Blueprints/IA_Move.IA_Move"))
  (:`Triggered`
    (`self.AddMovementInput` (`self.GetActorForwardVector`) ActionValue_X)
    (`self.AddMovementInput` (`self.GetActorRightVector`) ActionValue_Y)))

(event `EnhancedInput|/Game/Blueprints/IA_Look`
  (params (ActionValue :type "Vector2D Structure") (ElapsedSeconds :type "Float (double-precision)") (TriggeredSeconds :type "Float (double-precision)") (InputAction :type "InputAction Object Reference" :default "/Game/Blueprints/IA_Look.IA_Look"))
  (:`Triggered`
    (`self.AddControllerPitchInput` ActionValue_Y)
    (`self.AddControllerYawInput` ActionValue_X)))

(event `death`
  (`self.K2_SetActorTransform` (`self.startPos`))
  (set `self.health` 100.0))

(event `self.CapsuleComponent.OnComponentHit`
  (params (HitComponent :type "PrimitiveComponent Object Reference") (OtherActor :type "Actor Object Reference") (OtherComp :type "PrimitiveComponent Object Reference") (NormalImpulse :type "Vector Structure") (Hit :type "HitResult Structure (by ref)"))
  (bind _returnvalue (<= (`self.health`) 0.0))
  (if (`ActorComponent.ComponentHasTag` OtherComp "pain1")
    (set `self.health` (- (`self.health`) 15.0))
    (if _returnvalue
      (`self.death`))
    (elif (`ActorComponent.ComponentHasTag` OtherComp "pain2")
      (set `self.health` (- (`self.health`) 5.0))
      (if _returnvalue
        (`self.death`)))))

(fn `UserConstructionScript`)